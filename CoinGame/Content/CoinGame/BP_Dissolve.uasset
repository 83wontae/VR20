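; BP_Dissolve is an actor that plays a looping dissolve effect on its Cube component.
; The construction script creates a dynamic material instance from M_Dissolve_Inst, stores it and applies it to the cube.
; Tick steadily lowers a value over time, writes it to the "Dissolve" scalar parameter, and resets it once it drops slightly below zero.
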(event EventBeginPlay)

(event EventTick
  (params (DeltaSeconds :type Float%20%28single-precision%29))
  (Variables|Default|SetValue (- (Variables|Default|GetValue) (* DeltaSeconds 0.5)))
  (Rendering|Material|SetScalarParameterValue (Variables|Default|GetMaterialInst) "Dissolve" (Variables|Default|GetValue) :!class /Script/Engine.MaterialInstanceDynamic)
  (if (< (Variables|Default|GetValue) -0.1)
    (Variables|Default|SetValue 0.5)))

(fn ConstructionScript
  (bind _returnvalue (Rendering|Material|CreateDynamicMaterialInstance "/Game/Noise/M_Dissolve_Inst.M_Dissolve_Inst" "None" "Transient" :!class /Script/Engine.KismetMaterialLibrary))
  (Variables|Default|SetMaterialInst _returnvalue)
  (Rendering|Material|SetMaterial (Variables|Default|GetCube) 0 _returnvalue))