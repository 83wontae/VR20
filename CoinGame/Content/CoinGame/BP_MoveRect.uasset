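; BP_MoveRect is a coin game Blueprint that moves its Cube component around a square path in the local XZ plane while IsPlay is true.
; Tick switches on the MoveType state (Right, Up, Left, Down), stepping LocationX or LocationZ by a fixed amount and applying it as the relative location.
; Reaching a corner advances the state, so the loop repeats; steps ignore delta time, so speed depends on frame rate.
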(event EventTick
  (params (DeltaSeconds :type Float%20%28single-precision%29))
  (if (Variables|Default|GetIsPlay)
    (switch Utilities|FlowControl|Switch|SwitchonEN_MoveType (Variables|Default|GetMoveType)
      (:NewEnumerator0
        ;[1 1 1] 오른쪽으로 이동
        (bind _output_get (Variables|Default|SetLocationX (+ (Variables|Default|GetLocationX) 1.0)))
        (Transformation|SetRelativeLocation (Variables|Default|GetCube) (Math|Vector|MakeVector _output_get 0.0 (Variables|Default|GetLocationZ)) false false)
        (if (>= (.x (Variables|/Script/Engine.SceneComponent|GetRelativeLocation (Variables|Default|GetCube))) 1e+02)
          (Variables|Default|SetMoveType "NewEnumerator1")))
      (:NewEnumerator1
        ;[1 1 1] 위쪽으로 이동
        (bind _output_get_2 (Variables|Default|SetLocationZ (+ (Variables|Default|GetLocationZ) 1.0)))
        (Transformation|SetRelativeLocation (Variables|Default|GetCube) (Math|Vector|MakeVector (Variables|Default|GetLocationX) 0.0 _output_get_2) false false)
        (if (>= (.z (Variables|/Script/Engine.SceneComponent|GetRelativeLocation (Variables|Default|GetCube))) 1e+02)
          (Variables|Default|SetMoveType "NewEnumerator2")))
      (:NewEnumerator2
        ;[1 1 1] 왼쪽으로 이동
        (bind _output_get_3 (Variables|Default|SetLocationX (+ (Variables|Default|GetLocationX) -1.0)))
        (Transformation|SetRelativeLocation (Variables|Default|GetCube) (Math|Vector|MakeVector _output_get_3 0.0 (Variables|Default|GetLocationZ)) false false)
        (if (<= (.x (Variables|/Script/Engine.SceneComponent|GetRelativeLocation (Variables|Default|GetCube))) 0.0)
          (Variables|Default|SetMoveType "NewEnumerator3")))
      (:NewEnumerator3
        ;[1 1 1] 아래쪽으로 이동
        (bind _output_get_4 (Variables|Default|SetLocationZ (+ (Variables|Default|GetLocationZ) -1.0)))
        (Transformation|SetRelativeLocation (Variables|Default|GetCube) (Math|Vector|MakeVector (Variables|Default|GetLocationX) 0.0 _output_get_4) false false)
        (if (<= (.z (Variables|/Script/Engine.SceneComponent|GetRelativeLocation (Variables|Default|GetCube))) 0.0)
          (Variables|Default|SetMoveType "NewEnumerator0"))))))

(fn ConstructionScript)