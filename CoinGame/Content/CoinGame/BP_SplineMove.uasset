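; BP_SplineMove is a coin-game actor that moves a flattened cube continuously along a spline.
; Each Tick accumulates delta time scaled by Speed into a travelled distance.
; That distance, wrapped by the spline length, samples a world-space transform that sets the cube's location and rotation with a fixed thin scale, so it loops endlessly.
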(event EventTick
  (params (DeltaSeconds :type Float%20%28single-precision%29))
  (bind _spline (Variables|Default|GetSpline))
  (bind _output_get (Variables|Default|SetTotalDeltaSeconds (+ (* DeltaSeconds (Variables|Default|GetSpeed)) (Variables|Default|GetTotalDeltaSeconds))))
  (Transformation|SetWorldTransform (Variables|Default|GetCube) (Math|Transform|MakeTransform (.location (Spline|GetTransformatDistanceAlongSpline _spline (Math|Float|%(Float) _output_get (Spline|GetSplineLength _spline)) "World" false)) (.rotation (Spline|GetTransformatDistanceAlongSpline _spline (Math|Float|%(Float) _output_get (Spline|GetSplineLength _spline)) "World" false)) "1.000000,1.000000,0.100000") false false))

(fn ConstructionScript)