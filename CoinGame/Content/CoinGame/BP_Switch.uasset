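; BP_Switch is a trigger switch in CoinGame that turns other objects on while something overlaps its Cube.
; Begin overlap sets IsPlay to true on every entry in the LeftRight and MoveRect arrays, and end overlap sets it back to false.
; BeginPlay only prints index messages from two consecutive loops.
; An unconnected ForEach loop carries a Korean note explaining how that node works.
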(event OnComponentBeginOverlap(Cube)
  (params (OverlappedComponent :type Primitive%20Component%20Object%20Reference) (OtherActor :type Actor%20Object%20Reference) (OtherComp :type Primitive%20Component%20Object%20Reference) (OtherBodyIndex :type Integer) (bFromSweep :type Boolean) (SweepResult :type Hit%20Result%20Structure%20%28by%20ref%29))
  (for _array_element (Variables|Default|GetLeftRight)
    (Variables|/Game/CoinGame/BP_MoveLeftRight.BP_MoveLeftRight_C|SetIsPlay _array_element true))
  (for _array_element_2 (Variables|Default|GetMoveRect)
    (Variables|/Game/CoinGame/BP_MoveRect.BP_MoveRect_C|SetIsPlay _array_element_2 true)))

(event OnComponentEndOverlap(Cube)
  (params (OverlappedComponent :type Primitive%20Component%20Object%20Reference) (OtherActor :type Actor%20Object%20Reference) (OtherComp :type Primitive%20Component%20Object%20Reference) (OtherBodyIndex :type Integer))
  (for _array_element (Variables|Default|GetLeftRight)
    (Variables|/Game/CoinGame/BP_MoveLeftRight.BP_MoveLeftRight_C|SetIsPlay _array_element false))
  (for _array_element_2 (Variables|Default|GetMoveRect)
    (Variables|/Game/CoinGame/BP_MoveRect.BP_MoveRect_C|SetIsPlay _array_element_2 false)))

(event EventBeginPlay
  (for _index (range 1 5)
    (Development|PrintString (Utilities|String|Append "1st index - " (Utilities|String|ToString(Integer) _index)) true true "(R=0.000000,G=0.660000,B=1.000000,A=1.000000)" 6e+01))
  (for _index_2 (range 1 5)
    (Development|PrintString (Utilities|String|Append "2nd index - " (Utilities|String|ToString(Integer) _index_2)) true true "(R=0.000000,G=0.660000,B=1.000000,A=1.000000)" 6e+01)))

(fn ConstructionScript)