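; BP_Homing is an actor in the CoinGame folder that homes in on the first player's character.
; Each tick it moves along its Arrow component's forward vector at a constant speed, without sweeping for collision.
; It also eases its rotation toward the player with a look-at rotation and RInterpTo, so it turns gradually rather than snapping onto the target.
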(event EventBeginPlay)

(event Collision|EventActorBeginOverlap
  (params (OtherActor :type Actor%20Object%20Reference)))

(event EventTick
  (params (DeltaSeconds :type Float%20%28single-precision%29))
  (Transformation|AddActorWorldOffset (* (Math|Vector|GetForwardVector (Variables|Default|GetArrow)) (* DeltaSeconds 1e+02)))
  (Transformation|SetActorRotation (Math|Interpolation|RInterpTo (Transformation|GetActorRotation) (Math|Rotator|FindLookatRotation (Transformation|GetActorLocation) (Transformation|GetActorLocation (Game|GetPlayerCharacter 0))) DeltaSeconds 1.0)))

(fn ConstructionScript)