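; BP_MoveLeftRight is a coin-game actor whose Cube component slides back and forth along its relative X axis.
; Each Tick steps LocationX one unit up or down based on the Condition flag and applies it to the cube's relative location.
; The flag flips when the cube reaches either end of a 0 to 100 range, and movement is per frame without delta-time scaling.
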(event EventTick
  (params (DeltaSeconds :type Float%20%28single-precision%29))
  (if (Variables|Default|GetCondition)
    (bind _output_get (Variables|Default|SetLocationX (+ (Variables|Default|GetLocationX) 1.0)))
    (Transformation|SetRelativeLocation (Variables|Default|GetCube) (Math|Vector|MakeVector _output_get 0.0 0.0) false false)
    (if (>= (.x (Variables|/Script/Engine.SceneComponent|GetRelativeLocation (Variables|Default|GetCube))) 1e+02)
      (Variables|Default|SetCondition false))
    (else
      (bind _output_get_2 (Variables|Default|SetLocationX (+ (Variables|Default|GetLocationX) -1.0)))
      (Transformation|SetRelativeLocation (Variables|Default|GetCube) (Math|Vector|MakeVector _output_get_2 0.0 0.0) false false)
      (if (<= (.x (Variables|/Script/Engine.SceneComponent|GetRelativeLocation (Variables|Default|GetCube))) 0.0)
        (Variables|Default|SetCondition true)))))

(fn ConstructionScript)