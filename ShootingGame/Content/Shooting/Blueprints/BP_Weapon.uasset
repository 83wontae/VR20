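; Networked weapon actor that characters grab, drop, fire and reload, with mesh, damage, ammo and montages driven by WeaponData.
; Firing plays muzzle effects, then only the owning player sends a camera-aligned trace to the server, which spends ammo and damages hit BP_ShootingCharacters.
; Reload completion refills ammo locally, then requests a magazine from PlayerState.
; Ammo's OnRep raises a dispatcher that the local player's HUD binds on grab and unbinds on drop.
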(event Custom|ReqShoot
  (params (StartVector :type Vector) (EndVector :type Vector))
  ;[1 0 0] (Server)
  (bind _iscanshoot (CallFunction|IsCanShoot))
  (if _iscanshoot
    (CallFunction|UseAmmo)
    (bind _outhit (Collision|LineTraceForObjects StartVector EndVector (Utilities|Array|MakeArray "ObjectTypeQuery1" "ObjectTypeQuery2" "ObjectTypeQuery3" "ObjectTypeQuery4" "ObjectTypeQuery5" "ObjectTypeQuery6") false 0 "None"))
    (bind _asbp_shooting_character (Utilities|Casting|CastToBP_ShootingCharacter (.HitActor (Collision|BreakHitResult _outhit))))
    (Game|Damage|ApplyDamage _asbp_shooting_character (.Damage (Utilities|Struct|BreakST_WeaponData (Variables|Default|GetWeaponData))) (Pawn|GetController (Variables|Default|GetCharacter)) self)))

(event Custom|ReqReload
  (bind _asbp_shooting_player_state (Utilities|Casting|CastToBP_ShootingPlayerState (Variables|/Script/Engine.Pawn|GetPlayerState (Variables|Default|GetCharacter))))
  (bind _isuse_ (Default|UseMag _asbp_shooting_player_state))
  (if _isuse_
    (CallFunction|ChangeMag)))

(event EventBeginPlay
  (Components|StaticMesh|SetStaticMesh (Variables|Default|GetStaticMesh) (.StaticMesh (Utilities|Struct|BreakST_WeaponData (Variables|Default|GetWeaponData)))))

(fn ConstructionScript)

(fn CalcStartForwadVector
  (params (muzzleLoc :type Vector))
  (bind _returnvalue (Game|GetPlayerCameraManager 0))
  (bind _returnvalue_2 (Transformation|GetActorLocation _returnvalue))
  (bind _returnvalue_3 (Transformation|GetActorForwardVector _returnvalue))
  (return (+ _returnvalue_2 (* _returnvalue_3 (Math|Vector|Distance(Vector) muzzleLoc _returnvalue_2))) (+ _returnvalue_2 (* _returnvalue_3 5e+03))))

(fn OnRepAmmo
  (Default|CallEventDispatcherUpdateAmmo (Variables|Default|GetAmmo)))

(fn UseAmmo
  (Variables|Default|SetAmmo (- (Variables|Default|GetAmmo) 1)))

(fn BindAmmo
  (bind _returnvalue (Game|GetPlayerController 0))
  (if (== (Variables|Default|GetCharacter) (Pawn|GetControlledPawn _returnvalue))
    (bind _asbp_shooting_hud (Utilities|Casting|CastToBP_ShootingHud (HUD|GetHUD _returnvalue)))
    (Default|EventMyAmmo _asbp_shooting_hud (Variables|Default|GetAmmo))
    (EventDispatchers|BindEventtoEventDispatcherUpdateAmmo (EventDispatchers|CreateEvent _asbp_shooting_hud :!event EventMyAmmo))))

(fn UnBindAmmo
  (bind _returnvalue (Game|GetPlayerController 0))
  (if (== (Variables|Default|GetCharacter) (Pawn|GetControlledPawn _returnvalue))
    (bind _asbp_shooting_hud (Utilities|Casting|CastToBP_ShootingHud (HUD|GetHUD _returnvalue)))
    (EventDispatchers|UnbindEventfromEventDispatcherUpdateAmmo (EventDispatchers|CreateEvent _asbp_shooting_hud :!event EventMyAmmo))
    (Default|EventMyAmmo _asbp_shooting_hud)))

(fn ChangeMag
  (Variables|Default|SetAmmo (.MaxAmmo (Utilities|Struct|BreakST_WeaponData (Variables|Default|GetWeaponData)))))

(fn IsCanChangeMag
  (bind _character (Variables|Default|GetCharacter)
    (:then
      (bind _asbp_shooting_player_state (Utilities|Casting|CastToBP_ShootingPlayerState (Variables|/Script/Engine.Pawn|GetPlayerState _character))
        (:then
          (if (Default|IsCanUseMag _asbp_shooting_player_state)
            (return true)
            (else
              (return false))))
        (:CastFailed
          (return false))))
    (:else
      (return false))))

(fn GetShootDelaybyRPM
  (return (/ 1.0 (/ (.RPM (Utilities|Struct|BreakST_WeaponData (Variables|Default|GetWeaponData))) 60))))

(fn EventDrop
  (params (Character :type Character%20Object%20Reference))
  (bind _staticmesh (Variables|Default|GetStaticMesh))
  (CallFunction|UnBindAmmo)
  (Collision|SetCollisionEnabled _staticmesh "QueryAndPhysics")
  (Physics|SetSimulatePhysics _staticmesh true)
  (Transformation|DetachFromComponent _staticmesh "KeepWorld" "KeepWorld" "KeepWorld" true)
  (Variables|Default|SetCharacter 0)
  (return false))

(fn EventFire
  (bind _staticmesh (Variables|Default|GetStaticMesh))
  (bind _returnvalue (Transformation|GetSocketTransform _staticmesh "muzzle" "RTS_World"))
  (bind (_startvec _endvec) (CallFunction|CalcStartForwadVector (.location _returnvalue)))
  (bind _iscanshoot (CallFunction|IsCanShoot))
  (if _iscanshoot
    (Development|PrintString "Fire")
    (Effects|SpawnEmitteratLocation "/Game/StarterContent/Particles/P_Explosion.P_Explosion" (.location _returnvalue) (.rotation _returnvalue) "0.100000,0.100000,0.100000")
    (Audio|SpawnSoundatLocation "/Game/StarterContent/Audio/Explosion_Cue.Explosion_Cue" (.location _returnvalue) "0, 0, 0" 1.0 1.0 0.0 0 0)
    (Utilities|IsOwner?
      (:True
        (CallFunction|ReqShoot _startvec _endvec)
        (return true)))))

(fn EventGrab
  (params (Character :type Character%20Object%20Reference))
  (bind _staticmesh (Variables|Default|GetStaticMesh))
  (bind _output_get (Variables|Default|SetCharacter Character))
  (Physics|SetSimulatePhysics _staticmesh false)
  (Collision|SetCollisionEnabled _staticmesh "NoCollision")
  (Transformation|AttachComponentToComponent _staticmesh (Variables|/Script/Engine.Character|GetMesh _output_get) "weapon" "SnapToTarget" "SnapToTarget" "KeepWorld" true)
  (CallFunction|BindAmmo)
  (return (.WeaponType (Utilities|Struct|BreakST_WeaponData (Variables|Default|GetWeaponData)))))

(fn EventReload
  (Animation|PlayAnimMontage (Variables|Default|GetCharacter) (.ReloadMontage (Utilities|Struct|BreakST_WeaponData (Variables|Default|GetWeaponData))) 1.0 "None")
  (return false))

(fn EventReloadFinish
  (Utilities|IsOwner?
    (:True
      (if (CallFunction|IsCanChangeMag)
        (CallFunction|ChangeMag)
        (CallFunction|ReqReload)
        (return false)))))

(fn EventTigger
  (params (IsPressed :type Boolean))
  (bind _iscanshoot (CallFunction|IsCanShoot))
  (if _iscanshoot
    (if IsPressed
      (bind _character (Variables|Default|GetCharacter)
        (:then
          (Animation|PlayAnimMontage _character (.FireMontage (Utilities|Struct|BreakST_WeaponData (Variables|Default|GetWeaponData))) 1.0 "None")
          (return true))
        (:else)))))

(fn IsCanReload
  (return (and (< (Variables|Default|GetAmmo) (.MaxAmmo (Utilities|Struct|BreakST_WeaponData (Variables|Default|GetWeaponData)))) (!= (.ReloadMontage (Utilities|Struct|BreakST_WeaponData (Variables|Default|GetWeaponData))) (Animation|Montage|GetCurrentActiveMontage (Components|SkeletalMesh|GetAnimInstance (Variables|/Script/Engine.Character|GetMesh (Variables|Default|GetCharacter))))))))

(fn IsCanShoot
  (return (> (Variables|Default|GetAmmo) 0)))