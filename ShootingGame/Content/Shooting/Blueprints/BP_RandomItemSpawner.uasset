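; BP_RandomItemSpawner is a spawner actor that places a random item from its Items list at its own transform.
; BeginPlay calls SpawnItem, which runs only with authority and binds to the spawned actor's OnDestroyed event.
; EventItemDestroy sets a short fixed timer that calls SpawnItem again, so a new random item replaces the destroyed one.
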(event EventBeginPlay
  (CallFunction|SpawnItem))

(fn ConstructionScript)

(fn SpawnItem
  (bind _items (Variables|Default|GetItems))
  (Networking|SwitchHasAuthority
    (:Authority
      (if (Utilities|Array|IsNotEmpty _items)
        (bind _returnvalue (Game|SpawnActorfromClass (.OutItem (Utilities|Array|Random _items)) (Transformation|GetActorTransform) "Undefined" "MultiplyWithRoot" 0 0))
        (Game|BindEventtoOnDestroyed _returnvalue (EventDispatchers|CreateEvent :!event EventItemDestroy))))))

(fn EventItemDestroy
  (params (DestroyedActor :type Actor%20Object%20Reference))
  (Utilities|Time|SetTimerbyFunctionName 0 "SpawnItem" 5.0))