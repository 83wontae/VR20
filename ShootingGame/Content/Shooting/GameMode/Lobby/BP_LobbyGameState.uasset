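; Lobby game state that starts the match once all players are ready, moving the session to InGameMap.
; UpdateGameState, on authority only, checks every BP_LobbyPlayerState, then starts or cancels the countdown and resets its timer.
; Tick advances the five-second countdown, then locks the state and runs a servertravel console command.
; The state's RepNotify prints the new value and broadcasts it through an event dispatcher.
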(event EventTick
  (params (DeltaSeconds :type Float%20%28single-precision%29))
  (if (Utilities|Enum|Equal(Enum) (Variables|Default|GetGamsState) "NewEnumerator1")
    (bind _output_get (Variables|Default|SetCountDownDS (+ DeltaSeconds (Variables|Default|GetCountDownDS))))
    (if (> _output_get 5.0)
      (Variables|Default|SetCountDownDS 5.0)
      (Variables|Default|SetGamsState "NewEnumerator2")
      (CallFunction|DoMoveLevel))))

(fn ConstructionScript)

(fn CheckAllComplete
  (bind _outactors (Actor|GetAllActorsOfClass "/Game/Shooting/GameMode/Lobby/BP_LobbyPlayerState.BP_LobbyPlayerState_C"))
  (for _array_element _outactors
    (if (Utilities|Enum|NotEqual(Enum) (Variables|/Game/Shooting/GameMode/Lobby/BP_LobbyPlayerState.BP_LobbyPlayerState_C|GetLobbyState _array_element) "NewEnumerator1")
      (return false)))
  (return true))

(fn UpdateGameState
  (Networking|SwitchHasAuthority
    (:Authority
      (if (Utilities|Enum|NotEqual(Enum) (Variables|Default|GetGamsState) "NewEnumerator2")
        (if (CallFunction|CheckAllComplete)
          (Variables|Default|SetCountDownDS 0.0)
          (Variables|Default|SetGamsState "NewEnumerator1")
          (else
            (Variables|Default|SetCountDownDS 0.0)
            (Variables|Default|SetGamsState "NewEnumerator0")))))))

(fn DoMoveLevel
  (Development|ExecuteConsoleCommand "servertravel InGameMap" 0))

(fn OnRepGamsState
  (Development|PrintString (Utilities|String|Append "OnRepGameState - " (Utilities|String|EnumtoString (Variables|Default|GetGamsState))) true true "(R=0.000000,G=0.660000,B=1.000000,A=1.000000)" 6e+01)
  (Default|CallEventDispatcherGameState (Variables|Default|GetGamsState)))