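; Player controller for the shooting game's lobby that passes each player's locally stored user name to the server.
; On possession, the server calls ResOnPossess on the client, which reads UserName from BP_ShootingGameInst.
; The client returns it through the server event ReqNewUserName, which sets it on BP_LobbyPlayerState.
; Each step has a debug print with screen and log output turned off.
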(event Custom|ResOnPossess
  (params (Possessed%20Pawn :type Pawn%20Object%20Reference%20%28by%20ref%29))
  ;[1 1 1] (Client)
  (Development|PrintString (Utilities|String|Append "ResOnPossess Pawn - " (Utilities|GetDisplayName Possessed%20Pawn)) false false "(R=0.000000,G=0.660000,B=1.000000,A=1.000000)" 6e+01)
  (bind _asbp_shooting_game_inst (Utilities|Casting|CastToBP_ShootingGameInst (Game|GetGameInstance)))
  (CallFunction|ReqNewUserName (Variables|/Game/Shooting/GameMode/BP_ShootingGameInst.BP_ShootingGameInst_C|GetUserName _asbp_shooting_game_inst)))

(event Custom|ReqNewUserName
  (params (UserName :type String%20%28by%20ref%29))
  ;[1 0 0] (Server)
  (Development|PrintString (Utilities|String|Append "ReqNewUserName - " UserName) false false "(R=0.000000,G=0.660000,B=1.000000,A=1.000000)" 6e+01)
  (bind _asbp_lobby_player_state (Utilities|Casting|CastToBP_LobbyPlayerState (Variables|GetPlayerState)))
  (Default|SetUserName _asbp_lobby_player_state UserName))

(event EventPossess
  (params (PossessedPawn :type Pawn%20Object%20Reference))
  ;[1 0 0] (Server)
  (Development|PrintString (Utilities|String|Append "On Possess Pawn - " (Utilities|GetDisplayName PossessedPawn)) false false "(R=0.000000,G=0.660000,B=1.000000,A=1.000000)" 6e+01)
  (CallFunction|ResonPossess PossessedPawn))

(fn ConstructionScript)